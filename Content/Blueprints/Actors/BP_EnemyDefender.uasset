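; BP_EnemyDefender is an enemy actor that patrols back and forth along the Y axis around its spawn location.
; A looping Move timeline drives a swept SetActorLocation, scaling its YAxis curve by DistanceMovedInSecond and adding it to the saved start position.
; Each instance starts the timeline at a random playback position, so multiple defenders move out of sync.
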(event EventBeginPlay
  (Variables|Default|SetFirstLocation (Transformation|GetActorLocation))
  (Components|Timeline|SetPlaybackPosition (Variables|Default|GetMove) (Math|Random|RandomFloatinRange 0.0 2.0) false true)
  (bind _y_axis (Timeline|Move Play)
    (:Update
      (Transformation|SetActorLocation (Math|Vector|MakeVector (.x (Variables|Default|GetFirstLocation)) (+ (* _y_axis (Variables|Default|GetDistanceMovedInSecond)) (.y (Variables|Default|GetFirstLocation))) (.z (Variables|Default|GetFirstLocation))) true false))
    (:Finished
      (Timeline|Move PlayFromStart))))

(fn ConstructionScript)