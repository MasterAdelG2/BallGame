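; Game mode for a timed first-person score game, handling the main menu, game start, scoring, level restart and a persistent name-and-score leaderboard.
; BeginPlay loads the save and shows the menu; starting captures the player's name and swaps to the HUD.
; When time finishes, it unpossesses the player and saves new names or improved scores.
; A reverse bubble pass moves higher scores up, trimming past ten entries only when a swap occurs.
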(event Custom|OpenMainMenu
  (bind _returnvalue (Game|GetPlayerController 0))
  ;[1 1 1] Show MainMenu
  (Utilities|IsValid (Variables|Default|GetMainMenuRef)
    (:Is%20Valid
      _)
    (:Is%20Not%20Valid
      (bind _returnvalue_2 (UserInterface|CreateWidget "/Game/Blueprints/Widgets/WB_MainMenu.WB_MainMenu_C" _returnvalue (Variables|Default|GetLeaderBoard)))
      (Variables|Default|SetMainMenuRef _returnvalue_2)))
  (UserInterface|Viewport|AddtoViewport (Variables|Default|GetMainMenuRef) 0)
  (Input|SetInputModeUIOnly _returnvalue (Variables|Default|GetMainMenuRef) "DoNotLock")
  (Variables|/Script/Engine.PlayerController|SetbShowMouseCursor _returnvalue true)
  (Input|DisableInput (Game|Player|GetPlayerPawn 0) 0))

(event Custom|StartGame
  (bind _returnvalue (Game|GetPlayerController 0))
  (bind _mainmenuref (Variables|Default|GetMainMenuRef))
  ;[1 1 1] Start Game
  (Variables|Default|SetCurrentPName (Variables|/Game/Blueprints/Widgets/WB_MainMenu.WB_MainMenu_C|GetEnteredName _mainmenuref))
  (Widget|RemovefromParent _mainmenuref)
  (Variables|Default|SetCurrentPScore 0)
  (Utilities|IsValid (Variables|Default|GetHUDRef)
    (:Is%20Valid
      _)
    (:Is%20Not%20Valid
      (bind _returnvalue_2 (UserInterface|CreateWidget "/Game/Blueprints/Widgets/WB_MainHUD.WB_MainHUD_C" (Game|GetPlayerController 0) (.playerhighestscore (Utilities|Array|Get(acopy) (Variables|Default|GetLeaderBoard)))))
      (Variables|Default|SetHUDRef _returnvalue_2)))
  (UserInterface|Viewport|AddtoViewport (Variables|Default|GetHUDRef) 0)
  (Input|SetInputModeGameOnly _returnvalue)
  (Variables|/Script/Engine.PlayerController|SetbShowMouseCursor _returnvalue false)
  (Input|EnableInput (Game|Player|GetPlayerPawn 0) 0))

(event Custom|AddPointToScore
  ;[1 1 1] Add Score
  (bind _result (Math|Integer|IncrementInt (Variables|Default|GetCurrentPScore))
    (:%20%20
      (Variables|/Game/Blueprints/Widgets/WB_MainHUD.WB_MainHUD_C|SetPCurrentScore (Variables|Default|GetHUDRef) _result))))

(event Custom|TimeFinished
  ;[1 1 1] Update LeaderBoard
  (Audio|Components|Audio|Stop (Variables|/Script/StreamlineTest.StreamlineTestCharacter|GetJettingSFXSource (.AsFirst%20Person%20Character (Utilities|Casting|CastToFirstPersonCharacter (Game|Player|GetPlayerPawn 0)))))
  (Pawn|UnPossess (Game|GetPlayerController 0))
  (if (== (Utilities|Array|Length (Variables|Default|GetLeaderBoard)) 0)
    (Utilities|Array|Add (Variables|Default|GetLeaderBoard) (Utilities|Struct|MakeSPlayerScore (Variables|Default|GetCurrentPName) (Variables|Default|GetCurrentPScore)))
    (CallFunction|SortLeaderboard :!label _label)
    (CallFunction|SaveGame)
    (else
      (bind (_exist _iscurrenthigher _index) (CallFunction|CheckifNameExist))
      (if _exist
        (if _iscurrenthigher
          (Utilities|Array|SetArrayElem (Variables|Default|GetLeaderBoard) _index (Utilities|Struct|MakeSPlayerScore (Variables|Default|GetCurrentPName) (Variables|Default|GetCurrentPScore)))
          (goto _label))
        (else
          (Utilities|Array|Add (Variables|Default|GetLeaderBoard) (Utilities|Struct|MakeSPlayerScore (Variables|Default|GetCurrentPName) (Variables|Default|GetCurrentPScore)))
          (goto _label))))))

(event Custom|RestartLevel
  ;[1 1 1] RestartLevel
  (Game|OpenLevel(byName) "MainMap"))

(event EventBeginPlay
  ;[1 1 1] Check for Saves & Load MainMenu
  (CallFunction|SaveGameCheck)
  (CallFunction|OpenMainMenu))

(fn ConstructionScript)

(fn SaveGameCheck
  (bind _returnvalue (SaveGame|DoesSaveGameExist (Variables|Default|GetSaveSlotName)))
  (if _returnvalue
    (CallFunction|LoadGame)))

(fn SaveGame
  (Utilities|IsValid (Variables|Default|GetSaveGameRef)
    (:Is%20Valid
      _)
    (:Is%20Not%20Valid
      (bind _returnvalue (SaveGame|CreateSaveGameObject "/Game/Blueprints/BP_StreamlineSaveGame.BP_StreamlineSaveGame_C"))
      (Variables|Default|SetSaveGameRef _returnvalue)))
  (Variables|/Game/Blueprints/BP_StreamlineSaveGame.BP_StreamlineSaveGame_C|SetLeaderBoard (Variables|Default|GetSaveGameRef) (Variables|Default|GetLeaderBoard))
  (SaveGame|SaveGametoSlot (Variables|Default|GetSaveGameRef) (Variables|Default|GetSaveSlotName)))

(fn LoadGame
  (bind _returnvalue (SaveGame|LoadGamefromSlot (Variables|Default|GetSaveSlotName)))
  (bind _asbp_streamline_save_game (Utilities|Casting|CastToBP_StreamlineSaveGame _returnvalue))
  (Variables|Default|SetLeaderBoard (Variables|/Game/Blueprints/BP_StreamlineSaveGame.BP_StreamlineSaveGame_C|GetLeaderBoard _asbp_streamline_save_game)))

(fn CheckifNameExist
  (bind (_array_element _array_index) (Utilities|Array|ForEachLoopwithBreak (Variables|Default|GetLeaderBoard) :!label _label)
    (:LoopBody
      (if (Utilities|Enum|Equal(Enum) (.playername _array_element) (Variables|Default|GetCurrentPName))
        (goto _label Break)))
    (:Completed
      (return (Utilities|Enum|Equal(Enum) (.playername _array_element) (Variables|Default|GetCurrentPName)) (> (Variables|Default|GetCurrentPScore) (.playerhighestscore _array_element)) _array_index))))

(fn SortLeaderboard
  (bind _leaderboard (Variables|Default|GetLeaderBoard))
  (bind (_arrayindex _arrayelement) (Utilities|Array|ReverseforEachLoop (Variables|Default|GetLeaderBoard))
    (:LoopBody
      (if (!= _arrayindex 0)
        (if (> (.playerhighestscore _arrayelement) (.playerhighestscore (Utilities|Array|Get(acopy) _leaderboard (- _arrayindex 1))))
          (Utilities|Array|Swap _leaderboard _arrayindex (- _arrayindex 1))
          (if (> (Utilities|Array|Length _leaderboard) 10)
            (Utilities|Array|RemoveIndex _leaderboard 10)))))))